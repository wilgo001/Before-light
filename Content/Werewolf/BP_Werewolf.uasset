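; Werewolf actor Blueprint that adds periodic ambient wolf sounds on top of its parent class behavior.
; From BeginPlay, a self-calling custom event waits a random 15 to 60 seconds, plays the werewolf dash cue at the actor's location, then repeats indefinitely.
; Overlap and Tick events are disabled placeholders, and the construction script only calls the parent.
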(event Custom|PlayWolfSoundRandom
  (Utilities|FlowControl|Delay (Math|Random|RandomFloatinRange 15.0 6e+01))
  (Audio|PlaySoundatLocation "/Game/Sounds/Enfants/loup_garou_DASH_Cue.loup_garou_DASH_Cue" (Transformation|GetActorLocation) "0, 0, 0" 1.0 1.0 0.0 0 0 0)
  (CallFunction|PlayWolfSoundRandom))

(event EventBeginPlay
  (|CallParentFunction)
  (CallFunction|PlayWolfSoundRandom))

(event Collision|EventActorBeginOverlap
  (params (OtherActor :type Actor%20Object%20Reference)))

(event EventTick
  (params (DeltaSeconds :type Float%20%28single-precision%29))
  (|CallParentFunction DeltaSeconds) ; This node is disabled and will not be called.\nDrag off pins to build functionality.
)

(fn ConstructionScript
  (|CallParentFunction))