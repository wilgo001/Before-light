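; Save-data Blueprint that tracks the played level, story progress and a score for each of the Easy, Medium, Hard and Infinity levels.
; SetScoreForLevel overwrites only the score slot matching the played level.
; GetLevelConfig looks up that level in the Levels map and quits the game if it is missing.
; IncrementStoryLevel advances only from the current story level, setting fixed levels once the story list ends.
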(event Custom|SetScoreForLevel
  (params (score :type Integer))
  (switch Utilities|FlowControl|Switch|SwitchonLevelName (Variables|Default|GetplayedLevel)
    (:NewEnumerator6
      (Variables|Default|Setscores (Utilities|Struct|MakeScoreLevel (.leveleasy (Variables|Default|Getscores)) (.levelmedium (Variables|Default|Getscores)) (.levelhard (Variables|Default|Getscores)) score)))
    (:NewEnumerator7
      (Variables|Default|Setscores (Utilities|Struct|MakeScoreLevel score (.levelmedium (Variables|Default|Getscores)) (.levelhard (Variables|Default|Getscores)) (.levelinfinity (Variables|Default|Getscores)))))
    (:NewEnumerator8
      (Variables|Default|Setscores (Utilities|Struct|MakeScoreLevel (.leveleasy (Variables|Default|Getscores)) score (.levelhard (Variables|Default|Getscores)) (.levelinfinity (Variables|Default|Getscores)))))
    (:NewEnumerator9
      (Variables|Default|Setscores (Utilities|Struct|MakeScoreLevel (.leveleasy (Variables|Default|Getscores)) (.levelmedium (Variables|Default|Getscores)) score (.levelinfinity (Variables|Default|Getscores)))))))

(fn GetLevelConfig
  (bind _levels (Variables|Default|Getlevels))
  (bind _playedlevel (Variables|Default|GetplayedLevel))
  (bind (_value _returnvalue) (Utilities|Map|Find _levels _playedlevel))
  (if _returnvalue
    (return _value)
    (else
      (Game|QuitGame 0 0 "Quit" false))))

(fn IncrementStoryLevel
  (bind _storylevels (Variables|Default|GetstoryLevels))
  (if (Utilities|Enum|Equal(Enum) (Variables|Default|GetplayedLevel) (Variables|Default|GetstoryLevel))
    (if (>= (+ (Utilities|Array|FindItem _storylevels (Variables|Default|GetplayedLevel)) 1) (Utilities|Array|Length _storylevels))
      (Variables|Default|SetplayedLevel "NewEnumerator10")
      (Variables|Default|SetstoryLevel "NewEnumerator5")
      (else
        (bind _output_get (Variables|Default|SetplayedLevel (Utilities|Array|Get(acopy) _storylevels (+ (Utilities|Array|FindItem _storylevels (Variables|Default|GetplayedLevel)) 1))))
        (Variables|Default|SetstoryLevel _output_get)))
    (return)))