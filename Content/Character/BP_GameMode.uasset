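; Game mode that runs a countdown round and handles the win and fail screens.
; A self-repeating one-second timer decrements Seconds from BeginPlay and fires a sunrise call at thirty seconds left.
; When time runs out, it kills all child and vampire AI, plays child destroy animations, stops the music, plays a defeat sound and triggers GameFail.
; Fail and win each show their widget, reveal the cursor and pause the game.
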(event Custom|StartTimer
  (Utilities|FlowControl|Delay 1.0)
  (if (<= (Variables|Default|Getseconds) 0)
    (CallFunction|KillChilds)
    (else
      (bind _output_get (Variables|Default|Setseconds (- (Variables|Default|Getseconds) 1)))
      (if (== _output_get 30)
        (Default|CallStartSunRise))
      (CallFunction|StartTimer))))

(event Custom|GameFail
  (bind _returnvalue (UserInterface|CreateWidget "/Game/UIs/GameOverMenu/UI_GameOver.UI_GameOver_C"))
  (UserInterface|Viewport|AddtoViewport _returnvalue 1)
  (Variables|/Script/Engine.PlayerController|SetbShowMouseCursor (Game|GetPlayerController 0) true)
  (Game|SetGamePaused true))

(event Custom|GameWin
  (bind _returnvalue (UserInterface|CreateWidget "/Game/UIs/GameOverMenu/UI_GameWinStory.UI_GameWinStory_C"))
  (UserInterface|Viewport|AddtoViewport _returnvalue 1)
  (Variables|/Script/Engine.PlayerController|SetbShowMouseCursor (Game|GetPlayerController 0) true)
  (Game|SetGamePaused true))

(event Custom|KillChilds
  (bind _outactors (Actor|GetAllActorsOfClass "/Game/Child/AI_Child.AI_Child_C"))
  (for _array_element _outactors
    (Default|SetDead _array_element))
  (bind _outactors_2 (Actor|GetAllActorsOfClass "/Game/Vampire/AI_Vampire.AI_Vampire_C"))
  (for _array_element_2 _outactors_2
    (Default|SetDead _array_element_2))
  (bind _outactors_3 (Actor|GetAllActorsOfClass "/Game/Child/BP_Child.BP_Child_C"))
  (for _array_element_3 _outactors_3
    (Default|PlayDestroyAnimation _array_element_3))
  (Default|CallStopmusic)
  (Audio|PlaySound2D "/Game/Sounds/Defaite_V1.Defaite_V1" 1.0 1.0 0.0 0 0)
  (Utilities|FlowControl|Delay 1.0)
  (CallFunction|GameFail))

(event EventBeginPlay
  (CallFunction|StartTimer))

(fn ConstructionScript)