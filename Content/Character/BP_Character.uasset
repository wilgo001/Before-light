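; Player witch character that catches children and delivers them to a drop zone, winning through the GameMode at the target score.
; Axis input moves it and emits footstep sound plus AI noise; Tick flips and swaps flipbooks, and dash launches along velocity with cooldown.
; Sphere overlap marks catchable children; catching destroys the actor and shows a carry sprite, while dropping outside the zone respawns the stored class.
; Random laughs loop.
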(event OnComponentBeginOverlap(Sphere)
  (params (OverlappedComponent :type Primitive%20Component%20Object%20Reference) (OtherActor :type Actor%20Object%20Reference) (OtherComp :type Primitive%20Component%20Object%20Reference) (OtherBodyIndex :type Integer) (bFromSweep :type Boolean) (SweepResult :type Hit%20Result%20Structure%20%28by%20ref%29))
  ;[1 1 1] On Child Overlaping
  (bind _asbp_child (Utilities|Casting|CastToBP_Child OtherActor))
  (Default|ShowInteractSprite _asbp_child)
  (Variables|Default|SetNearChild _asbp_child)
  (Variables|Default|SethasNearChild true))

(event OnComponentEndOverlap(Sphere)
  (params (OverlappedComponent :type Primitive%20Component%20Object%20Reference) (OtherActor :type Actor%20Object%20Reference) (OtherComp :type Primitive%20Component%20Object%20Reference) (OtherBodyIndex :type Integer))
  ;[1 1 1] On Child Overlaping
  (bind _asbp_child (Utilities|Casting|CastToBP_Child OtherActor))
  (Default|HideInteractSprite _asbp_child)
  (Variables|Default|SethasNearChild false))

(event Custom|playRandomLaughSound
  (Utilities|FlowControl|Delay (Math|Random|RandomFloatinRange 1.0 6e+01))
  (Audio|PlaySoundatLocation "/Game/Sounds/Sorcière/Rire_Cue.Rire_Cue" (Transformation|GetActorLocation) "0, 0, 0" 0.7 1.0 0.0 0 0 0)
  (CallFunction|PlayRandomLaughSound))

(event Custom|PlaySound
  (bind _returnvalue (Transformation|GetActorLocation))
  ;[1 1 1] Play Footstep
  (Audio|PlaySoundatLocation "/Game/Character/ES_Footsteps_Dirt_21_-_SFX_Producer_Cue.ES_Footsteps_Dirt_21_-_SFX_Producer_Cue" _returnvalue "0, 0, 0" 0.5 1.0 0.0 0 0 0)
  (Class|AISenseHearing|ReportNoiseEvent _returnvalue 1.0 self 0.0 "Noise"))

(event Custom|DropChild
  ;[1 1 1] DropChild
  (Variables|Default|SethasCatchedChild false)
  (if (Variables|Default|GetisInDropZone)
    (Default|PlayAnimation (Variables|Default|GetDropingZone))
    (bind _result (Math|Integer|IncrementInt (Variables|Default|Getscore))
      (:%20%20
        (if (== _result (Variables|Default|GetscoreMax))
          (bind _asbp_game_mode (Utilities|Casting|CastToBP_GameMode (Game|GetGameMode)))
          (Default|GameWin _asbp_game_mode)
          (else
            (Rendering|SetVisibility (Variables|Default|GetPaperSprite) false false :!label _label)))))
    (else
      (AI|SpawnAIFromClass (Variables|Default|GetcatchedChild) 0 (+ (Transformation|GetActorLocation) "5.000000, 0,0.000000") "0, 0, 0" false 0)
      (goto _label))))

(event Custom|CatchChild
  (bind _nearchild (Variables|Default|GetNearChild))
  ;[1 1 1] Catch child
  (Variables|Default|SethasCatchedChild true)
  (Variables|Default|SetcatchedChild (Utilities|GetClass _nearchild))
  (Actor|DestroyActor _nearchild)
  (Rendering|SetVisibility (Variables|Default|GetPaperSprite) true false))

(event EventBeginPlay
  (Rendering|SetVisibility (Variables|Default|GetPaperSprite) false false)
  (CallFunction|PlayRandomLaughSound))

(event Collision|EventActorBeginOverlap
  (params (OtherActor :type Actor%20Object%20Reference)))

(event EventTick
  (params (DeltaSeconds :type Float%20%28single-precision%29))
  (bind _sprite (Variables|Default|GetSprite))
  (bind _sprite_2 (Variables|Default|GetSprite))
  (Utilities|FlowControl|Sequence
    (:then_0
      (Math|Float|CompareFloat (Math|Vector|DotProduct (Transformation|GetVelocity) (Transformation|GetActorForwardVector)) 0.0
        (:>
          (Transformation|SetRelativeRotation _sprite_2 "0,180.000000, 0" false false :!label _label))
        (:==
          (goto _label))
        (:<
          (Transformation|SetRelativeRotation _sprite_2 "0, 0, 0" false false))))
    (:then_1
      (if (Variables|Default|GetisDashing)
        (Sprite|SetFlipbook (Variables|Default|GetSprite) "/Game/Character/Anims/Witch_Dash_Frame.Witch_Dash_Frame")
        (elif (== (Math|Vector|VectorLengthSquared (Pawn|Components|CharacterMovement|GetCurrentAcceleration (Variables|Character|GetCharacterMovement))) 0.0)
          (Sprite|SetFlipbook _sprite "/Game/Character/Anims/Witch_Idle_Frame.Witch_Idle_Frame")
          (else
            (Sprite|SetFlipbook _sprite "/Game/Character/Anims/Witch_Walk_Frame.Witch_Walk_Frame")))))))

(event Input|ActionEvents|InputActionDash
  (params (Key :type Key%20Structure :default "None"))
  (bind _returnvalue (Transformation|GetVelocity))
  ;[1 1 1] Dash
  (:Pressed
    (if (Variables|Default|GetcanDash)
      (if (Math|Vector|NotEqual(Vector) _returnvalue "0, 0, 0" 0.0001)
        (Variables|Default|SetcanDash false)
        (Variables|Default|SetisDashing true)
        (Character|LaunchCharacter (* _returnvalue (Variables|Default|GetdashSpeed)) true true)
        (Utilities|FlowControl|Delay 0.25)
        (Variables|Default|SetisDashing false)
        (Utilities|FlowControl|Delay (Variables|Default|GetdashDelay))
        (Variables|Default|SetcanDash true)))))

(event Input|ActionEvents|InputActionInteract
  (params (Key :type Key%20Structure :default "None"))
  ;[1 1 1] Drop OR Catch child
  (:Pressed
    (if (Variables|Default|GethasCatchedChild)
      (CallFunction|DropChild)
      (elif (Variables|Default|GethasNearChild)
        (CallFunction|CatchChild)
        (Audio|PlaySoundatLocation "/Game/Sounds/Sorcière/attrapé_Cue.attrapé_Cue" (Transformation|GetActorLocation) "0, 0, 0" 0.7 1.0 0.0 0 0 0)))))

(event Input|AxisEvents|InputAxisMoveRight
  (params (AxisValue :type Float%20%28single-precision%29))
  ;[1 1 1] Movement
  (Pawn|Input|AddMovementInput "1.000000, 0, 0" AxisValue false)
  (if (!= AxisValue 0.0)
    (CallFunction|PlaySound)))

(event Input|AxisEvents|InputAxisMoveForward
  (params (AxisValue :type Float%20%28single-precision%29))
  ;[1 1 1] Movement
  (Pawn|Input|AddMovementInput "0,1.000000, 0" AxisValue false)
  (if (!= AxisValue 0.0)
    (CallFunction|PlaySound)))

(fn ConstructionScript)