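; BP_DropZone is a drop zone actor that tells BP_Character when it is inside and can play a firework celebration.
; Begin overlap sets the character's in-zone flag and hands it a reference to this zone, while end overlap clears only the flag.
; PlayAnimation, not called within this Blueprint, shows the hidden FireworkFrame, plays it once with a crackling sound, then hides it when playback finishes.
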(event OnFinishedPlaying(Firework_Frame)
  (bind _firework_frame (Variables|Default|GetFirework_Frame))
  (Audio|Components|Audio|Stop _firework_frame)
  (Rendering|SetVisibility _firework_frame false false))

(event Custom|PlayAnimation
  (bind _firework_frame (Variables|Default|GetFirework_Frame))
  (Rendering|SetVisibility _firework_frame true false)
  (Components|Timeline|PlayfromStart _firework_frame)
  (Audio|PlaySoundatLocation "/Game/Sounds/Fireworks-Crackling-www_fesliyanstudios_com_Cue.Fireworks-Crackling-www_fesliyanstudios_com_Cue" (Transformation|GetActorLocation) "0, 0, 0" 1.0 1.0 0.0 0 0 0))

(event EventBeginPlay
  (bind _firework_frame (Variables|Default|GetFirework_Frame))
  (Components|Timeline|SetLooping _firework_frame false)
  (Audio|Components|Audio|Stop _firework_frame)
  (Rendering|SetVisibility _firework_frame false false))

(event Collision|EventActorBeginOverlap
  (params (OtherActor :type Actor%20Object%20Reference))
  (bind _asbp_character (Utilities|Casting|CastToBP_Character OtherActor))
  (Variables|/Game/Character/BP_Character.BP_Character_C|SetisInDropZone _asbp_character true)
  (Variables|/Game/Character/BP_Character.BP_Character_C|SetDropingZone _asbp_character self))

(event EventTick
  (params (DeltaSeconds :type Float%20%28single-precision%29)))

(event Collision|EventActorEndOverlap
  (params (OtherActor :type Actor%20Object%20Reference))
  (bind _asbp_character (Utilities|Casting|CastToBP_Character OtherActor))
  (Variables|/Game/Character/BP_Character.BP_Character_C|SetisInDropZone _asbp_character false))

(fn ConstructionScript)