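; BP_Child is a 2D child character with flipbook animation, an interact prompt and a death animation.
; Tick locks actor rotation to zero and flips the sprite according to velocity along the forward vector.
; A self-recalling event plays a child voice cue at random intervals from BeginPlay onward.
; Events toggle the initially hidden prompt sprite, and PlayDestroyAnimation sets IsDead and plays the death flipbook once.
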(event Custom|HideInteractSprite
  (Rendering|SetVisibility (Variables|Default|GetPaperSprite) false false))

(event Custom|ShowInteractSprite
  (Rendering|SetVisibility (Variables|Default|GetPaperSprite) true false))

(event Custom|RandomSoundAtRandomTime
  (Utilities|FlowControl|Delay (Math|Random|RandomFloatinRange 1.0 9e+01))
  (Audio|PlaySoundatLocation "/Game/Sounds/Enfants/Na_NaNa__enfant__Cue.Na_NaNa__enfant__Cue" (Transformation|GetActorLocation) "0, 0, 0" 1.0 1.0 0.0 0 0 0)
  (CallFunction|RandomSoundatRandomTime))

(event EventTick
  (params (DeltaSeconds :type Float%20%28single-precision%29))
  (bind _sprite (Variables|Default|GetSprite))
  (Transformation|SetActorRotation "0, 0, 0")
  (Math|Float|CompareFloat (Math|Vector|DotProduct (Transformation|GetVelocity) (Transformation|GetActorForwardVector)) 0.0
    (:>
      (Transformation|SetRelativeRotation _sprite "0,180.000000, 0" false false :!label _label))
    (:==
      (goto _label))
    (:<
      (Transformation|SetRelativeRotation _sprite "0, 0, 0" false false))))

(event EventBeginPlay
  (Rendering|SetVisibility (Variables|Default|GetPaperSprite) false false)
  (CallFunction|RandomSoundatRandomTime))

(fn ConstructionScript)

(fn PlayDestroyAnimation
  (bind _sprite (Variables|Default|GetSprite))
  (bind _sprite_2 (Variables|Default|GetSprite))
  (Sprite|SetFlipbook _sprite "/Game/Child/Sprites/Death_Frame.Death_Frame")
  (Components|Timeline|SetLooping _sprite false)
  (Variables|Default|SetisDead true)
  (Audio|Components|Audio|Stop _sprite_2)
  (Components|Timeline|PlayfromStart _sprite_2)
  (return))