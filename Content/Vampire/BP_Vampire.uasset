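; Vampire actor Blueprint that handles the character's teleport/respawn explosion effects and periodic laugh sound.
; On begin play it hides its non-looping Explosion component, spawns a separate explosion actor and starts a self-recalling random-delay laugh loop.
; The respawn event plays the attached explosion, which hides itself when finished, while the position event plays the spawned actor at a given location, both with a teleport sound.
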(event OnFinishedPlaying(Explosion)
  (Rendering|SetVisibility (Variables|Default|GetExplosion) false false))

(event Custom|PlayExplosionOnPosition
  (params (position :type Vector))
  (Default|PlayatPosition (Variables|Default|GetexplosionActor) position)
  (Audio|PlaySoundatLocation "/Game/Sounds/Enfants/Tp_vampire_Cue.Tp_vampire_Cue" position "0, 0, 0" 1.0 1.0 0.0 0 0 0))

(event Custom|PlayExplosionRepawn
  (bind _explosion (Variables|Default|GetExplosion))
  (Rendering|SetVisibility _explosion true false)
  (Components|Timeline|PlayfromStart _explosion)
  (Audio|PlaySoundatLocation "/Game/Sounds/Enfants/Tp_vampire_Cue.Tp_vampire_Cue" (Transformation|GetActorLocation) "0, 0, 0" 1.0 1.0 0.0 0 0 0))

(event Custom|playVampSoundRandom
  (Utilities|FlowControl|Delay (Math|Random|RandomFloatinRange 15.0 6e+01))
  (Audio|PlaySoundatLocation "/Game/Sounds/Enfants/rire_vampire_1_Cue.rire_vampire_1_Cue" (Transformation|GetActorLocation) "0, 0, 0" 1.0 1.0 0.0 0 0 0)
  (CallFunction|PlayVampSoundRandom))

(event EventBeginPlay
  ;[1 1 1] Spawn explosion actor on begin play
  (|CallParentFunction)
  (Components|Timeline|SetLooping (Variables|Default|GetExplosion) false)
  (bind _returnvalue (Game|SpawnActorfromClass (Variables|Default|GetexplosionActorClass) (Transformation|GetActorTransform) "Undefined" 0 self))
  (Variables|Default|SetexplosionActor _returnvalue)
  (Rendering|SetVisibility (Variables|Default|GetExplosion) false false)
  (CallFunction|PlayVampSoundRandom))

(event Collision|EventActorBeginOverlap
  (params (OtherActor :type Actor%20Object%20Reference)))

(event EventTick
  (params (DeltaSeconds :type Float%20%28single-precision%29))
  (|CallParentFunction DeltaSeconds) ; This node is disabled and will not be called.\nDrag off pins to build functionality.
)

(fn ConstructionScript
  (|CallParentFunction))